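; Game instance Blueprint that handles LAN multiplayer sessions: hosting, finding and joining.
; Hosting creates a session, then opens "Level" as a listen server after short delays.
; Searches append servers with unseen names to a Sessions list, which is never cleared here, and print it.
; Joining first clears TeleportPlease on the player's FirstPersonCharacter; status and failures are reported only through debug prints.
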(event Custom|Instance_HostLobby
  (params (Host :type Player%20Controller%20Object%20Reference))
  (bind _output_get (Variables|Default|SetlastHost Host))
  (|Session _output_get 10 true
    (:then
      (Development|PrintString "CreatingSession" true true "(R=0.000000,G=0.660000,B=1.000000,A=1.000000)" 5.0))
    (:OnSuccess
      (Development|PrintString "Session Created" true true "(R=0.000000,G=1.000000,B=0.067597,A=1.000000)" 5.0)
      (Utilities|FlowControl|Delay 0.2)
      (Development|PrintString "Opening Level" true true "(R=0.000000,G=0.660000,B=1.000000,A=1.000000)" 5.0)
      (Utilities|FlowControl|Delay 0.2)
      (Game|OpenLevel(byName) "Level" true "listen"))
    (:OnFailure
      (Development|PrintString "session creation failed" true true "(R=1.000000,G=0.000000,B=0.072084,A=1.000000)" 5.0))))

(event Custom|Instance_JoinLobby
  (params (joining :type Player%20Controller%20Object%20Reference) (SessionToJoin :type Blueprint%20Session%20Result%20Structure))
  (bind _asfirst_person_character (Utilities|Casting|CastToFirstPersonCharacter (Pawn|GetControlledPawn joining)))
  (Variables|/Game/FirstPersonBP/Blueprints/FirstPersonCharacter.FirstPersonCharacter_C|SetTeleportPlease _asfirst_person_character false)
  (|JoinSession joining SessionToJoin
    (:OnFailure
      (Development|PrintString "Hello"))))

(event Custom|Instance_FindNewSessions
  (params (PlayerController :type Player%20Controller%20Object%20Reference))
  (bind _sessions (Variables|Default|GetSessions))
  (bind _results (|FindSessions PlayerController 10 true)
    (:OnSuccess
      (for _array_element _results
        (Variables|Default|Setfound false)
        ;[1 1 1] if the array of sessions contains the server, do not add it to the list
        (for _array_element_2 _sessions
          (if (Utilities|Enum|Equal(Enum) (Class|FindSessionsCallbackProxy|GetServerName _array_element_2) (Class|FindSessionsCallbackProxy|GetServerName _array_element))
            (Variables|Default|Setfound true)))
        (if (not (Variables|Default|Getfound))
          (Utilities|Array|Add _sessions _array_element)))
      (for (_array_element_3 _array_index) _sessions
        (Development|PrintString (Utilities|String|Append (Class|FindSessionsCallbackProxy|GetServerName _array_element_3) "  " (Utilities|String|ToString(Integer) _array_index) "                               " (Utilities|GetObjectName PlayerController)) true true "(R=1.000000,G=0.900370,B=0.008226,A=1.000000)" 1e+01)))
    (:OnFailure
      (Development|PrintString "Search Fail"))))